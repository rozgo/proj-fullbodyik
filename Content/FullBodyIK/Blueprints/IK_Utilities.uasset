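; IK_Utilities is a Full Body IK Blueprint utility whose DebugDrawCubicBezier function visualizes a cubic Bézier curve from four control points.
; It approximates the curve with a fixed count of short debug lines, sampling CubicBezier at evenly spaced steps.
; Two differently colored arrows show the tangent handles from each endpoint to its control point.
; The Time input is unused.
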(fn `DebugDrawCubicBezier`
  (params (Time :type "Float (double-precision)") (P0 :type "Vector Structure") (P1 :type "Vector Structure") (P2 :type "Vector Structure") (P3 :type "Vector Structure"))
  (bind _returnvalue (`KismetMathLibrary.Conv_IntToDouble` 30))
  (for _index (range 30)
    (`KismetSystemLibrary.DrawDebugLine` null (`DynamicalUtil.CubicBezier` (/ (`KismetMathLibrary.Conv_IntToDouble` _index) _returnvalue) P0 P1 P2 P3) (`DynamicalUtil.CubicBezier` (/ (`KismetMathLibrary.Conv_IntToDouble` (+ _index 1)) _returnvalue) P0 P1 P2 P3) (struct :`R` 1.0 :`G` 0.887345 :`A` 1.0) 0.0 0.0))
  (`|ExecutionSequence`
    (:`then_0`
      (`KismetSystemLibrary.DrawDebugArrow` null P0 P1 2.0 (struct :`R` 1.0 :`B` 0.654823 :`A` 1.0)))
    (:`then_1`
      (`KismetSystemLibrary.DrawDebugArrow` null P3 P2 2.0 (struct :`G` 0.573642 :`B` 1.0 :`A` 1.0)))))