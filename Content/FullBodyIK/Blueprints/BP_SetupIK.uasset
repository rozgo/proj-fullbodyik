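; BP_SetupIK feeds VR headset and motion controller transforms into the character's BP_FullBodyIK animation instance.
; It caches the anim instance on BeginPlay, then while enabled updates hand and head targets each tick by composing configurable offsets with the tracked actors' transforms.
; It also derives a mesh-relative head transform and a FABRIK target lowered along the HMD's up vector.
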(event `self.ReceiveBeginPlay`
  (bind _asbp_full_body_ik (cast `/Game/FullBodyIK/Characters/Mannequin/Blueprints/BP_FullBodyIK` (`SkeletalMeshComponent.GetAnimInstance` (`SkeletalMeshActor.SkeletalMeshComponent` (`self.Character`)))))
  (set `self.AnimInstance` _asbp_full_body_ik))

(event `self.ReceiveTick`
  (params (DeltaSeconds :type "Float (single-precision)"))
  (bind _animinstance (`self.AnimInstance`))
  (bind _animinstance_2 (`self.AnimInstance`))
  (bind (_returnvalue_location _returnvalue_rotation) (`KismetMathLibrary.BreakTransform` (`self.GetTransform` (`self.HMD`))))
  (bind _returnvalue (`KismetMathLibrary.ComposeTransforms` (`self.HeadOffset`) (`KismetMathLibrary.MakeTransform` _returnvalue_location _returnvalue_rotation)))
  (if (`self.Enabled`)
    (`|ExecutionSequence`
      (:`then_0`
        (set `/Game/FullBodyIK/Characters/Mannequin/Blueprints/BP_FullBodyIK.HandR` (`KismetMathLibrary.ComposeTransforms` (`self.HandOffsetR`) (`self.GetTransform` (`self.MotionControllerR`))) _animinstance))
      (:`then_1`
        (set `/Game/FullBodyIK/Characters/Mannequin/Blueprints/BP_FullBodyIK.HandL` (`KismetMathLibrary.ComposeTransforms` (`self.HandOffsetL`) (`self.GetTransform` (`self.MotionControllerL`))) _animinstance))
      (:`then_2`
        (set `/Game/FullBodyIK/Characters/Mannequin/Blueprints/BP_FullBodyIK.Head` _returnvalue _animinstance)
        (set `/Game/FullBodyIK/Characters/Mannequin/Blueprints/BP_FullBodyIK.LocalHead` (`KismetMathLibrary.ComposeTransforms` _returnvalue (`KismetMathLibrary.InvertTransform` (`SceneComponent.K2_GetComponentToWorld` (`AnimInstance.GetOwningComponent` _animinstance_2)))) (`self.AnimInstance`))
        (set `/Game/FullBodyIK/Characters/Mannequin/Blueprints/BP_FullBodyIK.FabrikTarget` (`KismetMathLibrary.ComposeTransforms` (`self.HeadOffset`) (`KismetMathLibrary.MakeTransform` (+ _returnvalue_location (* (`KismetMathLibrary.GetUpVector` _returnvalue_rotation) -10.0)) _returnvalue_rotation)) _animinstance_2)))))

(fn `UserConstructionScript`)