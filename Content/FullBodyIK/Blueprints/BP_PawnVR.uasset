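; VR pawn that drives a full-body IK character from headset and motion controller tracking.
; On BeginPlay it caches the child HMD and character actors and the character's BP_FullBodyIK anim instance.
; Each tick it copies the camera's relative transform onto the HMD actor and, when enabled, feeds offset hand, head, mesh-local head and lowered FABRIK targets to that instance.
; The construction script sets camera height by Oculus Rift or HTC Vive device.
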(event `self.ReceiveBeginPlay`
  (bind _asbp_hmd (cast `/Game/FullBodyIK/Blueprints/BP_HMD` (`ChildActorComponent.ChildActor` (`self.ChildHMD`))))
  (set `self.TargetHMD` _asbp_hmd)
  (bind _asbp_character (cast `/Game/FullBodyIK/Characters/Mannequin/BP_Character` (`ChildActorComponent.ChildActor` (`self.ChildCharacter`))))
  (set `self.BP_Character` _asbp_character)
  (bind _asbp_full_body_ik (cast `/Game/FullBodyIK/Characters/Mannequin/Blueprints/BP_FullBodyIK` (`SkeletalMeshComponent.GetAnimInstance` (`/Game/FullBodyIK/Characters/Mannequin/BP_Character.SkeletalMesh` (`self.BP_Character`)))))
  (set `self.AnimInstance` _asbp_full_body_ik)
  (`self.SetOwner` (`self.TargetHMD`) self))

(event `self.ReceiveTick`
  (params (DeltaSeconds :type "Float (single-precision)"))
  (bind _animinstance (`self.AnimInstance`))
  (bind _animinstance_2 (`self.AnimInstance`))
  (bind (_returnvalue_location _returnvalue_rotation) (`KismetMathLibrary.BreakTransform` (`self.GetTransform` (`self.TargetHMD`))))
  (bind _returnvalue (`KismetMathLibrary.ComposeTransforms` (`self.HeadOffset`) (`KismetMathLibrary.MakeTransform` _returnvalue_location _returnvalue_rotation)))
  (`self.K2_SetActorTransform` (`self.TargetHMD`) (`SceneComponent.GetRelativeTransform` (`self.Camera`)) false false)
  (if (`self.Enabled`)
    (`|ExecutionSequence`
      (:`then_0`
        (set `/Game/FullBodyIK/Characters/Mannequin/Blueprints/BP_FullBodyIK.HandR` (`KismetMathLibrary.ComposeTransforms` (`self.HandOffsetR`) (`self.GetTransform` (`ChildActorComponent.ChildActor` (`self.ChildMotionControllerR`)))) _animinstance))
      (:`then_1`
        (set `/Game/FullBodyIK/Characters/Mannequin/Blueprints/BP_FullBodyIK.HandL` (`KismetMathLibrary.ComposeTransforms` (`self.HandOffsetL`) (`self.GetTransform` (`ChildActorComponent.ChildActor` (`self.ChildMotionControllerL`)))) _animinstance))
      (:`then_2`
        (set `/Game/FullBodyIK/Characters/Mannequin/Blueprints/BP_FullBodyIK.Head` _returnvalue _animinstance)
        (set `/Game/FullBodyIK/Characters/Mannequin/Blueprints/BP_FullBodyIK.LocalHead` (`KismetMathLibrary.ComposeTransforms` _returnvalue (`KismetMathLibrary.InvertTransform` (`SceneComponent.K2_GetComponentToWorld` (`AnimInstance.GetOwningComponent` _animinstance_2)))) (`self.AnimInstance`))
        (set `/Game/FullBodyIK/Characters/Mannequin/Blueprints/BP_FullBodyIK.FabrikTarget` (`KismetMathLibrary.ComposeTransforms` (`self.HeadOffset`) (`KismetMathLibrary.MakeTransform` (+ _returnvalue_location (* (`KismetMathLibrary.GetUpVector` _returnvalue_rotation) -10.0)) _returnvalue_rotation)) _animinstance_2)))))

(fn `UserConstructionScript`
  (if (select `/Game/FullBodyIK/Miscellaneous/E_ListDevice` (`self.Device`) :`NewEnumerator0` true)
    (`SceneComponent.K2_SetRelativeLocation` (`self.Camera`) (0.0 0.0 177.0) false false)
    (else
      (`SceneComponent.K2_SetRelativeLocation` (`self.Camera`) (0.0 0.0 0.0) false false))))