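; IK_Debug_Player is a debug controller that drives the full-body IK pawn with simulated motion controller input.
; On BeginPlay it finds the first IK_Pawn in the level and possesses it.
; Each tick it moves the pawn's left motion controller child along a small time-based circle in the world XZ plane around a fixed point, using sine and cosine, and prints the sine value.
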(event `self.ReceiveBeginPlay`
  (bind _outactors (`GameplayStatics.GetAllActorsOfClass` "/Game/FullBodyIK/Blueprints/IK_Pawn.IK_Pawn_C"))
  (bind _output_get (set `self.IK_Pawn` (`|GetArrayItem` _outactors)))
  (`self.Possess` self _output_get))

(event `self.ReceiveTick`
  (params (DeltaSeconds :type "Float (single-precision)"))
  (bind _returnvalue (* (`KismetSystemLibrary.GetGameTimeInSeconds`) 180.0))
  (bind _returnvalue_2 (`KismetMathLibrary.DegSin` _returnvalue))
  (`/Engine/EditorBlueprintResources/StandardMacros.IsValid` (`self.IK_Pawn`)
    (:`Is Valid`
      (`SceneComponent.K2_SetWorldLocation` (`/Game/FullBodyIK/Blueprints/IK_Pawn.ChildMotionControllerL` (`self.IK_Pawn`)) (+ (* (`KismetMathLibrary.MakeVector` _returnvalue_2 0.0 (`KismetMathLibrary.DegCos` _returnvalue)) 10.0) (`KismetMathLibrary.MakeVector` 20.0 20.0 140.0)) false false)
      (`KismetSystemLibrary.PrintString` (`KismetStringLibrary.Conv_DoubleToString` _returnvalue_2)))))

(fn `UserConstructionScript`)