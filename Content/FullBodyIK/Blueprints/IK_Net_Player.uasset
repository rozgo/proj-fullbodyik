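; IK_Net_Player is a controller that represents a networked VR player as a full-body IK pawn.
; On BeginPlay it links its NetAvatar to the first NetClient in the level, then spawns an IK_Pawn and possesses it after a short delay.
; Each tick it copies NetAvatar's head and hand transforms onto the pawn's HMD and motion controller children, printing the HMD location for debugging.
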(event `self.ReceiveBeginPlay`
  (`|ExecutionSequence`
    (:`then_0`
      (bind _outactors (`GameplayStatics.GetAllActorsOfClass` "/Script/DynamicalSystems.NetClient"))
      (set `NetAvatar.NetClient` (`|GetArrayItem` _outactors) (`self.NetAvatar`)))
    (:`then_1`
      (bind _returnvalue (`|SpawnActorFromClass` "/Game/FullBodyIK/Blueprints/IK_Pawn.IK_Pawn_C" (`SceneComponent.K2_GetComponentToWorld` (`self.TransformComponent`)) "AlwaysSpawn" "OverrideRootScale"))
      (`KismetSystemLibrary.Delay` 0.2)
      (`|ExecutionSequence`
        (:`then_0`
          (`self.Possess` self _returnvalue))
        (:`then_1`
          (bind _output_get (set `self.IK_Pawn` _returnvalue)))))))

(event `self.ReceiveTick`
  (params (DeltaSeconds :type "Float (single-precision)"))
  (bind _netavatar (`self.NetAvatar`))
  (bind _netavatar_2 (`self.NetAvatar`))
  (bind _netavatar_3 (`self.NetAvatar`))
  (bind _locationhmd (`NetAvatar.LocationHMD` _netavatar))
  (`/Engine/EditorBlueprintResources/StandardMacros.IsValid` (`self.IK_Pawn`)
    (:`Is Valid`
      (`SceneComponent.K2_SetWorldTransform` (`/Game/FullBodyIK/Blueprints/IK_Pawn.ChildMotionControllerL` (`self.IK_Pawn`)) (`KismetMathLibrary.MakeTransform` (`NetAvatar.LocationHandL` _netavatar_3) (`NetAvatar.RotationHandL` _netavatar_3)) false false)
      (`SceneComponent.K2_SetWorldTransform` (`/Game/FullBodyIK/Blueprints/IK_Pawn.ChildMotionControllerR` (`self.IK_Pawn`)) (`KismetMathLibrary.MakeTransform` (`NetAvatar.LocationHandR` _netavatar_2) (`NetAvatar.RotationHandR` _netavatar_2)) false false)
      (`SceneComponent.K2_SetWorldTransform` (`/Game/FullBodyIK/Blueprints/IK_Pawn.ChildHMD` (`self.IK_Pawn`)) (`KismetMathLibrary.MakeTransform` _locationhmd (`NetAvatar.RotationHMD` _netavatar)) false false)
      (`KismetSystemLibrary.PrintString` (`KismetStringLibrary.Conv_VectorToString` _locationhmd)))))

(fn `UserConstructionScript`)