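; VR pawn that drives a full-body IK character from the headset and two motion controllers.
; Each tick it estimates center of mass on a debug-drawn cubic Bézier between HMD and pawn root, which slowly follows it horizontally.
; Offset head and hand transforms plus center of mass feed the child character's IK_Animation instance.
; A spawned body actor's proportional-only PID controller targets center of mass, supplying the animation's velocity input.
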(event `self.ReceiveBeginPlay`
  (`|ExecutionSequence`
    (:`then_0`
      (`self.SetOwner` (`ChildActorComponent.ChildActor` (`self.ChildHMD`)) self))
    (:`then_1`
      (bind _asik_character (cast `/Game/FullBodyIK/Characters/Mannequin/IK_Character` (`ChildActorComponent.ChildActor` (`self.ChildCharacter`))))
      (set `self.Character` _asik_character)
      (bind _asik_animation (cast `/Game/FullBodyIK/Characters/Mannequin/Blueprints/IK_Animation` (`SkeletalMeshComponent.GetAnimInstance` (`/Game/FullBodyIK/Characters/Mannequin/IK_Character.SkeletalMesh` (`self.Character`)))))
      (set `self.AnimInstance` _asik_animation))
    (:`then_2`
      (`self.SetupTransforms`))))

(event `self.ReceiveTick`
  (params (DeltaSeconds :type "Float (single-precision)"))
  (bind _velocityarrowhmd (`self.VelocityArrowHMD`))
  (bind _defaultsceneroot (`self.DefaultSceneRoot`))
  (bind (_returnvalue_x _returnvalue_y _returnvalue_z) (`KismetMathLibrary.BreakVector` (`SceneComponent.K2_GetComponentLocation` _defaultsceneroot)))
  (bind _returnvalue (`self.K2_GetActorLocation` (`ChildActorComponent.ChildActor` (`self.ChildHMD`))))
  (bind (_returnvalue_x_2 _returnvalue_y_2) (`KismetMathLibrary.BreakVector` (`SceneComponent.K2_GetComponentLocation` (`/Game/FullBodyIK/Blueprints/IK_Transform.DefaultSceneRoot` (`self.CenterOfMass`)))))
  (bind _returnvalue_2 (- _returnvalue (`self.LastLocationHMD`)))
  (`|ExecutionSequence`
    (:`then_1`
      (if (> (`KismetMathLibrary.VSize` _returnvalue_2) 0.1)
        (`SceneComponent.K2_SetWorldRotation` _velocityarrowhmd (`KismetMathLibrary.MakeRotFromX` _returnvalue_2) false false)
        (`SceneComponent.K2_SetWorldLocation` _velocityarrowhmd (+ (`SceneComponent.K2_GetComponentLocation` (`/Game/FullBodyIK/Blueprints/IK_Transform.DefaultSceneRoot` (`self.CenterOfMass`))) (0.0 0.0 20.0)) false false)))
    (:`then_2`
      (`self.UpdateTransforms`))
    (:`then_3`
      (`self.ApplyTransforms`))
    (:`then_4`
      (set `self.LastLocationHMD` _returnvalue))
    (:`then_5`
      (`SceneComponent.K2_SetWorldLocation` (`self.DefaultSceneRoot`) (`KismetMathLibrary.VInterpTo` (`SceneComponent.K2_GetComponentLocation` _defaultsceneroot) (`KismetMathLibrary.MakeVector` _returnvalue_x_2 _returnvalue_y_2 _returnvalue_z) DeltaSeconds 1.0) false false))))

(fn `SetBodyColor`
  (params (Color :type "LinearColor Structure"))
  (bind _returnvalue (`PrimitiveComponent.CreateDynamicMaterialInstance` (`self.GetComponentByClass` (`ChildActorComponent.ChildActor` (`self.ChildCharacter`)) "/Script/Engine.SkinnedMeshComponent") 0 "/Game/FullBodyIK/Characters/Mannequin/Materials/MI_FullBody.MI_FullBody"))
  (`MaterialInstanceDynamic.SetVectorParameterValue` _returnvalue "BodyColor" Color))

(fn `UserConstructionScript`
  (if (select `/Game/FullBodyIK/Miscellaneous/E_ListDevice` (`self.Device`) :`NewEnumerator0` true)
    (`SceneComponent.K2_SetRelativeLocation` (`self.VROrigin`) (0.0 0.0 175.0) false false)
    (else
      (`SceneComponent.K2_SetRelativeLocation` (`self.VROrigin`) (0.0 0.0 0.0) false false))))