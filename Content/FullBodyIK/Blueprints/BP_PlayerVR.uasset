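; BP_PlayerVR is a VR player Blueprint that drives the controller components of a BP_PawnVR in a full-body IK setup.
; On BeginPlay it caches the first BP_PawnVR found in the level.
; Every tick it applies the relative transforms of its left and right motion controllers as world transforms on that pawn's child controller components, without adding its own actor transform.
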(event `self.ReceiveBeginPlay`
  (bind _outactors (`GameplayStatics.GetAllActorsOfClass` "/Game/FullBodyIK/Blueprints/BP_PawnVR.BP_PawnVR_C"))
  (set `self.BP_PawnVR` (`|GetArrayItem` _outactors)))

(event `self.ReceiveTick`
  (params (DeltaSeconds :type "Float (single-precision)"))
  (bind _bp_pawnvr (`self.BP_PawnVR`))
  (`SceneComponent.K2_SetWorldTransform` (`/Game/FullBodyIK/Blueprints/BP_PawnVR.ChildMotionControllerL` _bp_pawnvr) (`SceneComponent.GetRelativeTransform` (`self.MotionControllerL`)) false false)
  (`SceneComponent.K2_SetWorldTransform` (`/Game/FullBodyIK/Blueprints/BP_PawnVR.ChildMotionControllerR` _bp_pawnvr) (`SceneComponent.GetRelativeTransform` (`self.MotionControllerR`)) false false))

(fn `UserConstructionScript`)