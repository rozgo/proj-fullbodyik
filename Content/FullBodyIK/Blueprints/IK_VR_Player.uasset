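; IK_VR_Player is a VR player Blueprint that feeds tracking transforms to an IK_Pawn for full-body IK.
; On BeginPlay it finds the first IK_Pawn in the level and caches its IK_HMD child actor.
; Each Tick it sets the pawn's child controllers' world transforms from its own motion controllers' relative transforms.
; The pawn's child HMD follows the world transform of that pawn's camera.
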(event `self.ReceiveBeginPlay`
  (bind _outactors (`GameplayStatics.GetAllActorsOfClass` "/Game/FullBodyIK/Blueprints/IK_Pawn.IK_Pawn_C"))
  (bind _output_get (set `self.IK_Pawn` (`|GetArrayItem` _outactors)))
  (bind _asik_hmd (cast `/Game/FullBodyIK/Blueprints/IK_HMD` (`ChildActorComponent.ChildActor` (`/Game/FullBodyIK/Blueprints/IK_Pawn.ChildHMD` _output_get))))
  (set `self.IK_HMD` _asik_hmd))

(event `self.ReceiveTick`
  (params (DeltaSeconds :type "Float (single-precision)"))
  (`/Engine/EditorBlueprintResources/StandardMacros.IsValid` (`self.IK_Pawn`)
    (:`Is Valid`
      (`SceneComponent.K2_SetWorldTransform` (`/Game/FullBodyIK/Blueprints/IK_Pawn.ChildMotionControllerL` (`self.IK_Pawn`)) (`SceneComponent.GetRelativeTransform` (`self.MotionControllerL`)) false false)
      (`SceneComponent.K2_SetWorldTransform` (`/Game/FullBodyIK/Blueprints/IK_Pawn.ChildMotionControllerR` (`self.IK_Pawn`)) (`SceneComponent.GetRelativeTransform` (`self.MotionControllerR`)) false false)
      (`SceneComponent.K2_SetWorldTransform` (`/Game/FullBodyIK/Blueprints/IK_Pawn.ChildHMD` (`self.IK_Pawn`)) (`SceneComponent.K2_GetComponentToWorld` (`/Game/FullBodyIK/Blueprints/IK_Pawn.Camera` (`self.IK_Pawn`))) false false))))

(fn `UserConstructionScript`)