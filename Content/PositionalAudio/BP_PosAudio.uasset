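; BP_PosAudio is a placeable positional audio source for one stem of a VeniceStream music stream.
; On BeginPlay it finds the first VeniceStream actor and sets its Master track volume to zero.
; Each Tick it passes the player camera's transform, its Cube's location and a min/max range to that stream's OVR positional parameters for the chosen Stem.
; The construction script labels it with the stem's name, leaving secondary stems blank.
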(event `self.ReceiveBeginPlay`
  (bind _outactors (`GameplayStatics.GetAllActorsOfClass` "/Script/Venice.VeniceStream"))
  (bind _output_get (set `self.VS` (`|GetArrayItem` _outactors)))
  (`VeniceStream.SetTrackVolumeParams` _output_get "Master" 0.0))

(event `self.ReceiveTick`
  (params (DeltaSeconds :type "Float (single-precision)"))
  (bind _returnvalue (`self.GetComponentByClass` (`GameplayStatics.GetPlayerPawn` 0) "/Script/Engine.CameraComponent"))
  (`VeniceStream.SetOVRPositionalParams` (`self.VS`) (`self.Stem`) (`self.RangeMin`) (`self.RangeMax`) (`SceneComponent.K2_GetComponentLocation` _returnvalue) (`SceneComponent.K2_GetComponentRotation` _returnvalue) (`SceneComponent.K2_GetComponentLocation` (`self.Cube`))))

(fn `UserConstructionScript`
  (`TextRenderComponent.K2_SetText` (`self.TextRender`) (`KismetTextLibrary.Conv_StringToText` (select `EStemNames` (`self.Stem`) :`Master` "Master" :`DrumsPrimary` "Rhythm" :`BassPrimary` "Bass" :`MelodyPrimary` "Melody" :`VocalPrimary` "Vocal"))))